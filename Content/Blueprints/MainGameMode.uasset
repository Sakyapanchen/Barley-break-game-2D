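; Game mode that boots the main HUD and handles restart and victory flow.
; On BeginPlay it forces an 800x800 resolution through a console command, adds MainHUD to the viewport and sets Game and UI input focused on it.
; A restart event, called from MainPlayerController, restarts the game.
; A victory event, called from MainHUD, creates and displays the VictoryScreen widget.
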(event Custom|RestartGameEvent
  ;[1 1 1] Restart
  (Class|GameMode|RestartGame))

(event Custom|VictoryEvent
  ;[1 1 1] Victory
  (bind _returnvalue (UserInterface|CreateWidget "/Game/Blueprints/VictoryScreen.VictoryScreen_C"))
  (bind _output_get (Variables|Default|SetvictoryScreenRef _returnvalue))
  (UserInterface|Viewport|AddtoViewport _output_get 0))

(event EventBeginPlay
  ;[1 1 1] Begin game
  (Development|ExecuteConsoleCommand "r.SetRes 800x800")
  (bind _returnvalue (UserInterface|CreateWidget "/Game/Blueprints/MainHUD.MainHUD_C"))
  (UserInterface|Viewport|AddtoViewport _returnvalue 0)
  (Input|SetInputModeGameandUI (Game|GetPlayerController 0) _returnvalue false false))

(fn ConstructionScript)